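; Gameplay ability for a melee attack that plays the goblin spear attack montage and damages nearby live players.
; On activation, the avatar turns toward its combat target through CombatInterface, then waits for the montage's attack gameplay event.
; That event triggers a small radius query at the combat socket, damages each player found and ends the ability.
; Montage completion and interruption are unhandled, so ending relies on that event once the montage starts.
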(event `self.K2_ActivateAbility`
  (bind _avator_actor (`self.Avator Actor`))
  (set `self.Avator Actor` (`self.GetAvatarActorFromActorInfo`))
  (bind _returnvalue (message `EnemyInterface.GetCombatTarget` (`self.Avator Actor`)))
  (bind _ascombat_interface (cast `CombatInterface` (`self.Avator Actor`))
    (:`then`
      (`CombatInterface.UpdateFacingTarget` _ascombat_interface (`Actor.K2_GetActorLocation` _returnvalue))
      (`AbilityTask_PlayMontageAndWait.CreatePlayMontageAndWaitProxy` "None" "/Game/Assets/Enemies/Goblin/Animations/Spear/AM_Attack_GoblinSpear.AM_Attack_GoblinSpear"
        (:`then`
          (`AbilityTask_WaitGameplayEvent.WaitGameplayEvent` (struct :`TagName` "Event.Montage.Attack") null
            (:`EventReceived`
              (bind _returnvalue_2 (message `CombatInterface.GetCombatSocketLocation` _avator_actor))
              (bind _outoverlappingactors (`AuraAbilitySystemLibrary.GetLivePlayersWithinRadius` _avator_actor (`|MakeArray` _avator_actor) 45.0 _returnvalue_2))
              (for _array_element _outoverlappingactors
                (`self.CauseDamage` _array_element))
              (`self.K2_EndAbility`))))))
    (:`CastFailed`
      (`self.K2_EndAbility`))))