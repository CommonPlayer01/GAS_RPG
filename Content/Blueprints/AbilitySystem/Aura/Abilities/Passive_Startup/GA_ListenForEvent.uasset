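; Passive gameplay ability that converts Attributes gameplay events into an event-based Gameplay Effect on its owner.
; On activation it prints a debug string, waits for events under the Attributes tag hierarchy, and stores each payload's tag and magnitude.
; MakeGESpechandle builds the effect spec, gives the exactly matching EventTags entry the magnitude via SetByCaller, zeroes the others, then applies it to self.
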(event `self.K2_ActivateAbility`
  (`KismetSystemLibrary.PrintString` "ListenForEvent" true true (struct :`R` 0.138126 :`G` 1.0 :`B` 0.341871 :`A` 1.0))
  (bind (_asynctaskproxy _payload) (`AbilityTask_WaitGameplayEvent.WaitGameplayEvent` (struct :`TagName` "Attributes") null false false)
    (:`EventReceived`
      (bind (_eventtag _instigator _target _optionalobject _optionalobject2 _contexthandle _instigatortags _targettags _eventmagnitude) (break `GameplayEventData` _payload))
      (set `self.Event Tag` _eventtag)
      (set `self.Event Magnitude` _eventmagnitude)
      (`self.MakeGESpechandle`))))

(fn `MakeGESpechandle`
  (bind _returnvalue (`self.GetAbilitySystemComponentFromActorInfo`))
  (set `self.GESpec` (`AbilitySystemComponent.MakeOutgoingSpec` _returnvalue (`self.EventBasedEffectClass`) 1.0 (`AbilitySystemComponent.MakeEffectContext` _returnvalue)))
  (for _array_element (`self.EventTags`)
    (if (`BlueprintGameplayTagLibrary.MatchesTag` (`self.Event Tag`) _array_element true)
      (`AbilitySystemBlueprintLibrary.AssignTagSetByCallerMagnitude` (`self.GESpec`) (`self.Event Tag`) (`self.Event Magnitude`))
      (else
        (`AbilitySystemBlueprintLibrary.AssignTagSetByCallerMagnitude` (`self.GESpec`) _array_element))))
  (`AbilitySystemComponent.BP_ApplyGameplayEffectSpecToSelf` (`self.GetAbilitySystemComponentFromActorInfo`) (`self.GESpec`)))