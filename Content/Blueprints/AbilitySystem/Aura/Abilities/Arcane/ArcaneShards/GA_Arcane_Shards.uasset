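; Gameplay ability that casts Arcane Shards, a series of radial-damage bursts around a targeted ground point.
; It shows a magic circle, then on press takes the point under the mouse and spawns a point collection for level-based, capped, randomly rotated shard locations.
; A montage event starts a looping timer that damages nearby live players and fires a GameplayCue per shard.
; Cost commits at the first shard, cooldown after the last.
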(event `self.K2_ActivateAbility`
  (`self.K2_CheckAbilityCost`)
  (`|ExecutionSequence`
    (:`then_0`
      (message `PlayerInterface.ShowMagicCircle` (`self.GetAvatarActorFromActorInfo`) null))
    (:`then_1`
      ; 接收到press事件后,获取鼠标位置生成pointcollection
      (`AbilityTask_WaitInputPress.WaitInputPress` false
        (:`OnPress`
          (bind (_asynctaskproxy _datahandle) (`TargetDataUnderMouse.CreateTargetDataUnderMouse`)
            (:`ValidData`
              (set `self.Impact Point` (`.ImpactPoint` (`GameplayStatics.BreakHitResult` (`AbilitySystemBlueprintLibrary.GetHitResultFromTargetData` _datahandle))))
              (`|ExecutionSequence`
                (:`then_0`
                  (bind _returnvalue (`|SpawnActorFromClass` "/Game/Blueprints/AbilitySystem/Aura/Abilities/Arcane/ArcaneShards/BP_PointCollection.BP_PointCollection_C" (`KismetMathLibrary.MakeTransform` (`self.Impact Point`)) "Undefined" "MultiplyWithRoot" null null))
                  (set `self.PointCollection` _returnvalue)
                  (set `self.Num Shards` (`KismetMathLibrary.Min` (`self.MaxNumShards`) (`self.GetAbilityLevel`)))
                  (set `self.Ground Points` (`PointCollection.GetGroundPoints` (`self.PointCollection`) (`self.Impact Point`) (`self.Num Shards`) (`KismetMathLibrary.RandomFloatInRange` 0.0 360.0))))
                (:`then_1`
                  ; 更新角色转向
                  (message `CombatInterface.UpdateFacingTarget` (`self.GetAvatarActorFromActorInfo`) (`self.Impact Point`)))
                (:`then_2`
                  ; 播放montage并等待事件
                  (`AbilityTask_PlayMontageAndWait.CreatePlayMontageAndWaitProxy` "None" "/Game/Assets/Characters/Aura/Animations/Abilities/AM_Cast_ArcaneShards.AM_Cast_ArcaneShards"
                    (:`then`
                      (`AbilityTask_WaitGameplayEvent.WaitGameplayEvent` (struct :`TagName` "Event.Montage.ArcaneShards") null true
                        (:`EventReceived`
                          ; 设置定时任务并产生第一个碎片
                          (set `self.Index` 0)
                          (bind _returnvalue_2 (`KismetSystemLibrary.K2_SetTimerDelegate` (delegate `SpawnShard`) (`self.Shard Spawn Time`) true))
                          (set `self.Spawn Timer Handle` _returnvalue_2)
                          (message `PlayerInterface.HideMagicCircle` (`self.GetAvatarActorFromActorInfo`))
                          (`self.SpawnShard`)
                          (`self.K2_CommitAbilityCost` false))))))))))))))

(event `SpawnShard`
  (`|ExecutionSequence`
    (:`then_0`
      (`self.StoreShardSpawnLocation`))
    (:`then_1`
      ; 获取附近存活目标 并遍历造成伤害
      (`self.StorePlayersToDamage`)
      (for _array_element (`self.PlayersToDamage`)
        (`self.RadialDamageToPlayer` _array_element))
      ; 播放GameplayCue 并判断是否结束技能
      (`self.K2_ExecuteGameplayCueWithParams` (struct :`TagName` "GameplayCue.ArcaneShards") (`AbilitySystemBlueprintLibrary.MakeGameplayCueParameters` 0.0 0.0 (struct) (struct) (struct) (struct) (struct) (`self.Shard Spawn Location`)))
      (bind _result (`/Engine/EditorBlueprintResources/StandardMacros.IncrementInt` (`self.Index`))
        (:`  `
          (if (>= _result (`self.Num Shards`))
            (`self.K2_CommitAbilityCooldown` false)
            (`self.K2_EndAbility`)))))))

(event `self.K2_OnEndAbility`
  (params (bWasCancelled :type Boolean))
  (bind _pointcollection (`self.PointCollection`)
    (:`then`
      (`Actor.K2_DestroyActor` _pointcollection)
      (`KismetSystemLibrary.K2_ClearAndInvalidateTimerHandle` (`self.Spawn Timer Handle`)))
    (:`else`)))

(fn `RadialDamageToPlayer`
  (params (TargetActor :type "Actor Object Reference"))
  (`AuraAbilitySystemLibrary.ApplyDamageEffect` (`self.MakeDamageEffectParamsFromClassDefaults` TargetActor (`self.Shard Spawn Location`))))

(fn `StorePlayersToDamage`
  (bind _returnvalue (`self.GetAvatarActorFromActorInfo`))
  (bind _outoverlappingactors (`AuraAbilitySystemLibrary.GetLivePlayersWithinRadius` _returnvalue (`|MakeArray` _returnvalue) (`self.RadialDamageOuterRadius`) (`self.Shard Spawn Location`)))
  (set `self.PlayersToDamage` _outoverlappingactors))

(fn `StoreShardSpawnLocation`
  (returns (Output_Get :type "Vector Structure"))
  (bind _output_get (set `self.Shard Spawn Location` (`SceneComponent.K2_GetComponentLocation` (`|GetArrayItem` (`self.Ground Points`) (`self.Index`)))))
  (return _output_get))