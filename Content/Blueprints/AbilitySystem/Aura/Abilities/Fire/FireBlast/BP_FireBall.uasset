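; Fireball projectile for the FireBlast ability that flies out along its forward vector, then homes back to ReturnToActor and explodes.
; On the server, StartOutgoingTimeline runs an outgoing timeline to the apex, then a returning timeline that lerps toward the actor's current location.
; Within ExplodeDistance it calls OnHit, applies radial damage effect params to live players in radius except its owner, and destroys itself.
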(event `self.StartOutgoingTimeline`
  (bind _returnvalue (`self.GetOwner`))
  (bind _array (`|MakeArray` _returnvalue))
  (`/Engine/EditorBlueprintResources/ActorMacros.Switch Has Authority`
    (:`Authority`
      ; 存储初始位置和顶点位置
      (set `self.Initial Location` (`self.K2_GetActorLocation`))
      (set `self.Apex Location` (+ (`self.Initial Location`) (* (`self.GetActorForwardVector`) (`self.Travel Distance`))))
      (bind (_direction _outgoingtrack) (`Timeline|OutgoingTimeline`)
        (:`Update`
          (`self.K2_SetActorLocation` (`KismetMathLibrary.VLerp` (`self.Initial Location`) (`self.Apex Location`) _outgoingtrack)))
        (:`Finished`
          (bind (_direction_2 _returningtrack) (`Timeline|ReturningTimeline`)
            (:`Update`
              (`self.K2_SetActorLocation` (`KismetMathLibrary.VLerp` (`self.Apex Location`) (`self.K2_GetActorLocation` (`self.ReturnToActor`)) _returningtrack))
              (if (`self.IsWithinExplodeDistance`)
                (`self.OnHit`)
                ; 获取附近敌人并应用伤害
                (`KismetArrayLibrary.Array_Add` _array _returnvalue)
                (bind _outoverlappingactors (`AuraAbilitySystemLibrary.GetLivePlayersWithinRadius` self _array (`self.RadialDamageOuterRadius`) (`self.K2_GetActorLocation`)))
                (set `self.OverlappingPlayers` _outoverlappingactors)
                (`AuraAbilitySystemLibrary.SetIsRadialDamageEffectParams` (`self.ExplosionDamageParams`) true (`self.RadialDamageInnerRadius`) (`self.RadialDamageOuterRadius`) (`self.K2_GetActorLocation`))
                (for _array_element (`self.OverlappingPlayers`)
                  (`AuraAbilitySystemLibrary.SetEffectParamsTargetASC` (`self.ExplosionDamageParams`) (`AbilitySystemBlueprintLibrary.GetAbilitySystemComponent` _array_element))
                  (`AuraAbilitySystemLibrary.ApplyDamageEffect` (`self.ExplosionDamageParams`)))
                (`self.K2_DestroyActor`)))))))))

(fn `IsWithinExplodeDistance`
  (returns (ReturnValue :type Boolean))
  (return (<= (`KismetMathLibrary.VSize` (- (`self.K2_GetActorLocation`) (`self.K2_GetActorLocation` (`self.ReturnToActor`)))) (`self.ExplodeDistance`))))

(fn `UserConstructionScript`)