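; GA_Ranged_Attack is an enemy gameplay ability that fires a projectile at the avatar's combat target.
; On activation it fetches the target through interface messages, updates the avatar's facing toward it, and picks a random tagged attack montage.
; It plays that montage, waits once for the gameplay event matching the montage's tag to spawn the projectile at the target's location, and ends when the montage completes.
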(event `self.K2_ActivateAbility`
  (`|ExecutionSequence`
    (:`then_0`
      (bind _output_get (set `self.AvatorActor` (`self.GetAvatarActorFromActorInfo`)))
      (bind _returnvalue (message `EnemyInterface.GetCombatTarget` _output_get))
      (set `self.CombatTarget` _returnvalue))
    (:`then_1`
      ; 获取随机montage
      (message `CombatInterface.UpdateFacingTarget` (`self.AvatorActor`) (`Actor.K2_GetActorLocation` (`self.CombatTarget`)))
      (bind _returnvalue_2 (message `CombatInterface.GetAttackMontages` (`self.AvatorActor`)))
      (bind (_montage _montagetag) (break `TaggedMontage` (`self.GetRandomTaggedMontageFromArray` _returnvalue_2)))
      (set `self.RandomMontage` _montage)
      (set `self.Montage Tag` _montagetag))
    (:`then_2`
      (`AbilityTask_PlayMontageAndWait.CreatePlayMontageAndWaitProxy` "None" (`self.RandomMontage`) 1.0 "None" false
        (:`then`
          (`AbilityTask_WaitGameplayEvent.WaitGameplayEvent` (`self.Montage Tag`) null true
            (:`EventReceived`
              (`self.SpawnProjectile` (`Actor.K2_GetActorLocation` (`self.CombatTarget`))))))
        (:`OnCompleted`
          (`self.K2_EndAbility`))))))