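; Enemy melee Gameplay Ability that turns the avatar toward its combat target and damages non-friendly actors within the strike area.
; It plays a random tagged attack montage from the combat interface and waits for that montage's gameplay event.
; On the event, it runs a small radius query at the tag's combat socket, applies damage, then ends without stopping the montage.
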(event `self.K2_ActivateAbility`
  (bind _avator_actor (`self.Avator Actor`))
  (set `self.Avator Actor` (`self.GetAvatarActorFromActorInfo`))
  (bind _returnvalue (message `EnemyInterface.GetCombatTarget` (`self.Avator Actor`)))
  (bind _ascombat_interface (cast `CombatInterface` (`self.Avator Actor`))
    (:`then`
      (`CombatInterface.UpdateFacingTarget` _ascombat_interface (`Actor.K2_GetActorLocation` _returnvalue))
      (bind _returnvalue_2 (message `CombatInterface.GetAttackMontages` (`self.Avator Actor`)))
      (bind _returnvalue_3 (`KismetArrayLibrary.Array_Length` _returnvalue_2))
      (bind _output_get (set `self.TaggedMontage` (`|GetArrayItem` _returnvalue_2 (`KismetMathLibrary.RandomIntegerInRange` (- _returnvalue_3 1)))))
      (if (> _returnvalue_3 0)
        (bind (_montage _montagetag) (break `TaggedMontage` _output_get))
        (`AbilityTask_PlayMontageAndWait.CreatePlayMontageAndWaitProxy` "None" _montage 1.0 "None" false
          (:`then`
            (`AbilityTask_WaitGameplayEvent.WaitGameplayEvent` _montagetag null
              (:`EventReceived`
                ; 寻找攻击生效范围内的目标 造成伤害
                (bind _returnvalue_4 (message `CombatInterface.GetCombatSocketLocation` _avator_actor _montagetag))
                (bind _outoverlappingactors (`AuraAbilitySystemLibrary.GetLivePlayersWithinRadius` _avator_actor (`|MakeArray` _avator_actor) 45.0 _returnvalue_4))
                (for _array_element _outoverlappingactors
                  (if (`AuraAbilitySystemLibrary.IsNotFriend` (`self.Avator Actor`) _array_element)
                    (`self.CauseDamage` _array_element)))
                (`self.K2_EndAbility`)))))
        (else
          (`self.K2_EndAbility`))))
    (:`CastFailed`
      (`self.K2_EndAbility`))))