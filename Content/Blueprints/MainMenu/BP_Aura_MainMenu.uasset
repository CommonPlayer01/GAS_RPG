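; BP_Aura_MainMenu is the main menu scene actor that runs the menu and its ambient animation.
; On BeginPlay it plays menu music, creates the BP_MainMenu widget, switches to UI-only input and shows the cursor.
; Tick accumulates time to bob the fireball vertically on an amplitude-scaled sine around its starting location, while rolling the magic circle decal at a configurable rate.
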(event `self.ReceiveBeginPlay`
  (bind _returnvalue (`GameplayStatics.GetPlayerController` 0))
  (set `self.FireBall Initial Location` (`SceneComponent.K2_GetComponentLocation` (`self.FireBall`)))
  (`GameplayStatics.PlaySound2D` "/Game/Assets/Sounds/Music/Music_MainMenu.Music_MainMenu" 1.0 1.0 0.0 null null)
  (bind _returnvalue_2 (`|CreateWidget` "/Game/Blueprints/UI/MainMenu/BP_MainMenu.BP_MainMenu_C"))
  (`UserWidget.AddToViewport` _returnvalue_2 0)
  (`WidgetBlueprintLibrary.SetInputMode_UIOnlyEx` _returnvalue _returnvalue_2)
  (set `PlayerController.bShowMouseCursor` true _returnvalue))

(event `self.ReceiveTick`
  (params (DeltaSeconds :type "Float (single-precision)"))
  (bind _output_get (`self.UpdateTime` DeltaSeconds))
  (`SceneComponent.K2_SetWorldLocation` (`self.FireBall`) (+ (`self.FireBall Initial Location`) (`KismetMathLibrary.MakeVector` 0.0 0.0 (`self.SinTime` _output_get))) false false)
  (`SceneComponent.K2_AddLocalRotation` (`self.MagicCircleDecal`) (`KismetMathLibrary.MakeRotator` (* (`GameplayStatics.GetWorldDeltaSeconds`) (`self.Magic Circle Rotation Rate`))) false false))

(fn `SinTime`
  (params (A :type "Float (double-precision)"))
  (returns (ReturnValue :type "Float (double-precision)"))
  (return (* (`KismetMathLibrary.Sin` A) (`self.Amplitude`))))

(fn `UpdateTime`
  (params (A :type "Float (double-precision)"))
  (returns (Output_Get :type "Float (single-precision)"))
  (bind _output_get (set `self.Time` (+ A (`self.Time`))))
  (return _output_get))

(fn `UserConstructionScript`)